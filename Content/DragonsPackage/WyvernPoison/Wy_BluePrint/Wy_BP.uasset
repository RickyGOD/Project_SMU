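; Poison wyvern enemy Blueprint that runs AI behavior and keeps turning to face the player.
; BeginPlay starts the Wy_BehaviorTree on the wyvern's AI controller.
; Tick interpolates the actor's rotation toward player character 0, taking only roll and yaw from the look-at rotation so pitch stays level.
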(event EventBeginPlay
  (AI|RunBehaviorTree (AI|GetAIController self) "/Game/DragonsPackage/WyvernPoison/Wy_BH/Wy_BehaviorTree.Wy_BehaviorTree"))

(event Collision|EventActorBeginOverlap
  (params (OtherActor :type Actor%20Object%20Reference)))

(event EventTick
  (params (DeltaSeconds :type Float%20%28single-precision%29))
  (bind _returnvalue (Transformation|GetActorLocation))
  (bind _returnvalue_2 (Game|GetPlayerCharacter 0))
  (bind _returnvalue_3 (Transformation|GetActorLocation _returnvalue_2))
  (bind _returnvalue_4 (Math|Rotator|FindLookatRotation _returnvalue _returnvalue_3))
  ;[1 1 1] 转向
  (Transformation|SetActorRotation (Math|Interpolation|RInterpTo (Transformation|GetActorRotation) (Math|Rotator|MakeRotator (.roll _returnvalue_4) 0.0 (.yaw _returnvalue_4)) DeltaSeconds 0.0)))

(fn ConstructionScript)