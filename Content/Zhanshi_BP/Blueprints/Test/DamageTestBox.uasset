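; DamageTestBox is a test damage volume that repeatedly hurts a Zhanshi-BP character while it overlaps.
; Begin overlap casts to Zhanshi-BP, sets IsInVolume and calls TakeDamage5, then repeats through a half-second Delay loop while the flag holds.
; End overlap from any actor clears the flag, since it does not check which actor left.
; An alternative looping box-trace ApplyDamage chain is left unconnected and never runs.
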(event EventBeginPlay)

(event Collision|EventActorBeginOverlap
  (params (OtherActor :type Actor%20Object%20Reference))
  (bind _aszhanshi__bp (Utilities|Casting|CastToZhanshi-BP OtherActor))
  (Variables|Default|SetIsInVolume true)
  (Default|TakeDamage5% _aszhanshi__bp :!label _label)
  (if (Variables|Default|GetIsInVolume)
    (Utilities|FlowControl|Delay 0.5)
    (goto _label)))

(event EventTick
  (params (DeltaSeconds :type Float%20%28single-precision%29)))

(event Collision|EventActorEndOverlap
  (params (OtherActor :type Actor%20Object%20Reference))
  (Variables|Default|SetIsInVolume false))

(fn ConstructionScript)