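; Barghest enemy creature that chases and attacks the Zhanshi player, then drops a blue ball on death.
; PawnSensing feeds the behavior tree's blackboard, and the attack event plays one of two random montages, notifying the task afterward while a hitbox overlap applies damage.
; Incoming hits look up damage from the player's weapon, attack or skill state, update the health widget, and play a hit reaction or trigger death once.
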(event OnComponentBeginOverlap(barghesthitboxcollision)
  (params (OverlappedComponent :type Primitive%20Component%20Object%20Reference) (OtherActor :type Actor%20Object%20Reference) (OtherComp :type Primitive%20Component%20Object%20Reference) (OtherBodyIndex :type Integer) (bFromSweep :type Boolean) (SweepResult :type Hit%20Result%20Structure%20%28by%20ref%29))
  ;[1 1 1] 伤害事件
  (if (Variables|Default|Geton%20attack%20player%20)
    (bind _aszhanshi__bp (Utilities|Casting|CastToZhanshi-BP OtherActor))
    (Game|Damage|ApplyDamage _aszhanshi__bp (Variables|Default|Getdamage01) 0 0)))

(event OnSeePawn(PawnSensing)
  (params (Pawn :type Pawn%20Object%20Reference))
  (bind _returnvalue (AI|GetBlackboard 0))
  ;[1 1 1] 看到玩家和把seen player和player变量获取到行为树
  (if (Actor|ActorHasTag Pawn "zhanshi tag")
    (Variables|Default|Setseen%20player true)
    (AI|Components|Blackboard|SetValueasBool _returnvalue (Utilities|Name|MakeLiteralName "seen player") true)
    (AI|Components|Blackboard|SetValueasObject _returnvalue (Utilities|Name|MakeLiteralName "player") Pawn)
    (Variables|/Script/Engine.CharacterMovementComponent|SetMaxWalkSpeed (Variables|Character|GetCharacterMovement) 5e+02)))

(event Custom|barghest_attack
  (params (task%20barghestattack :type Task%20Barghestattack%20Object%20Reference))
  (bind _returnvalue (Transformation|GetActorLocation))
  ;[1 1 1] 攻击事件
  (Transformation|SetActorRotation (Math|Rotator|FindLookatRotation (Math|Rotator|GetRotationXVector (Math|Rotator|MakeRotfromXY _returnvalue _returnvalue)) (Transformation|GetActorLocation (Game|GetPlayerCharacter 0))))
  (switch int (Math|Random|RandomIntegerinRange 0 1)
    (:0
      (Variables|Default|Seton%20attack%20player%20 true)
      (Variables|Default|Setattack%20montage "/Game/QuadrapedCreatures/Barghest/Blueprint/Montage/barghest_attack02.barghest_attack02"))
    (:1
      (Variables|Default|Seton%20attack%20player%20 true)
      (Variables|Default|Setattack%20montage "/Game/QuadrapedCreatures/Barghest/Blueprint/Montage/barghest_attack01.barghest_attack01")))
  (Animation|PlayAnimMontage (Variables|Default|Getattack%20montage) 1.0 "None")
  (Utilities|FlowControl|Delay (Variables|/Script/Engine.AnimSequenceBase|GetSequenceLength (Variables|Default|Getattack%20montage)))
  (Default|BarghestOnattack task%20barghestattack))

(event Custom|is%20dead
  ;[1 1 1] 死亡
  (bind _output_get (Variables|Default|Setisdead true))
  (AI|Components|Blackboard|SetValueasBool (AI|GetBlackboard 0) (Utilities|Name|MakeLiteralName "isdead") _output_get)
  (Collision|SetCollisionEnabled (Variables|Collision|GetCapsuleComponent) "NoCollision")
  (Utilities|FlowControl|Delay 3.0)
  (Actor|DestroyActor)
  ;[1 1 1] 死亡掉落蓝白球
  (Game|SpawnActorfromClass "/Game/QuadrapedCreatures/Barghest/Blueprint/Barghest_blueball.Barghest_blueball_C" (Math|Conversions|ToTransform(Vector) (Transformation|GetActorLocation)) "Undefined" 0 0))

(event EventBeginPlay
  (Variables|Default|SetHP (Variables|Default|GetMAX%20HP))
  ;[1 1 1] 获取变量到行为树
  (CallFunction|UpdateWidget)
  (AI|RunBehaviorTree (AI|GetAIController self) "/Game/QuadrapedCreatures/Barghest/Blueprint/Barghest_behaviorTree.Barghest_behaviorTree")
  (AI|Components|Blackboard|SetValueasFloat (AI|GetBlackboard 0) (Utilities|Name|MakeLiteralName "attackrange") (Variables|Default|Getattackrange)))

(event EventDamage
  (params (Aistate :type A%20Istate%20Structure) (Hitnumber :type Integer) (mageAistate :type Mage%20A%20Istate%20Structure) (GBLAistate :type GBLA%20Istate%20Structure) (BearAistate :type Bear%20A%20Istate%20Structure) (JYGAistate :type JYGA%20Istate%20Structure) (LXCAistate :type LXCA%20Istate%20Structure) (island1Aistate :type Island%201A%20Istate%20Structure) (island2Aistate :type Island%202A%20Istate%20Structure) (gouAistate :type Gou%20A%20Istate%20Structure) (island3Aistate :type Island%203A%20Istate%20Structure))
  ;[1 1 1 1 50] 受伤判断
  ;;[1 1 1] 判断具体攻击行为
  (bind _aszhanshi__bp (Utilities|Casting|CastToZhanshi-BP (Game|GetPlayerCharacter 0)))
  (if (Variables|/Game/Zhanshi_BP/Blueprints/Zhanshi-BP.Zhanshi-BP_C|GetIsGreatSword? _aszhanshi__bp)
    ;;[1 1 1] 左键伤害
    (switch int (Variables|/Game/Zhanshi_BP/Blueprints/Zhanshi-BP.Zhanshi-BP_C|GetNumber _aszhanshi__bp)
      (:0
        _)
      (:1
        _)
      (:2
        _)
      (:3
        _))
    (bind _damage (Default|StuckZhanShi _aszhanshi__bp "2Lattack"))
    (Utilities|Shsz _damage)
    (elif (Variables|/Game/Zhanshi_BP/Blueprints/Zhanshi-BP.Zhanshi-BP_C|Getleftkey _aszhanshi__bp)
      ;;[1 1 1] 左键伤害
      (switch int (Variables|/Game/Zhanshi_BP/Blueprints/Zhanshi-BP.Zhanshi-BP_C|GetNumber _aszhanshi__bp)
        (:0
          _)
        (:1
          _)
        (:2
          _)
        (:3
          _))
      (bind _damage_2 (Default|StuckZhanShi _aszhanshi__bp "1Lattack"))
      (Utilities|Shsz _damage_2)
      (elif (Variables|/Game/Zhanshi_BP/Blueprints/Zhanshi-BP.Zhanshi-BP_C|GetUsing%20SKILL _aszhanshi__bp)
        (if (Variables|/Game/Zhanshi_BP/Blueprints/Zhanshi-BP.Zhanshi-BP_C|GetE-Skill _aszhanshi__bp)
          ;;[1 1 1] E技能伤害
          (bind _skilldamage (Default|StuckZhanShi _aszhanshi__bp "ESkill"))
          (Utilities|Shsz _skilldamage)
          (elif (Variables|/Game/Zhanshi_BP/Blueprints/Zhanshi-BP.Zhanshi-BP_C|GetDunchong _aszhanshi__bp)
            (bind _skilldamage_2 (Default|StuckZhanShi _aszhanshi__bp "Dunchong"))
            (Utilities|Shsz _skilldamage_2)
            (else
              ;;[1 1 1] Q技能伤害
              (bind _skilldamage_3 (Default|StuckZhanShi _aszhanshi__bp "QSkill"))
              (Utilities|Shsz _skilldamage_3))))
        (else
          ;;[1 1 1] 右键伤害
          (switch int (Variables|/Game/Zhanshi_BP/Blueprints/Zhanshi-BP.Zhanshi-BP_C|GetNumber _aszhanshi__bp)
            (:0
              _)
            (:1
              _)
            (:2
              _)
            (:3
              _))
          (bind _damage_3 (Default|StuckZhanShi _aszhanshi__bp "1Rattack"))
          (Utilities|Shsz _damage_3)))))
  (CallFunction|UpdateWidget)
  ;;[1 1 1] 判断血量是否为0
  (Math|Float|CompareFloat (Variables|Default|GetHP) 0.0
    (:>
      (Animation|StopAnimMontage 0)
      ;;[1 1 1] 播放受伤动画
      (Animation|PlayAnimMontage (Utilities|Array|Get(acopy) (Utilities|Struct|BreakGBLAIstate GBLAistate) Hitnumber) 1.0 "None"))
    (:==
      (Utilities|FlowControl|DoOnce false :!label _label
        (:Completed
          (CallFunction|IsDead))))
    (:<
      (goto _label))))

(fn ConstructionScript)

(fn UpdateWidget
  (bind _asgouhealth_ui (Utilities|Casting|CastTogouhealthUI (UserInterface|GetUserWidgetObject (Variables|Default|GetgouWidget))))
  (Progress|SetPercent (Variables|/Game/UI/gouhealthUI.gouhealthUI_C|GetProgressBar_gou _asgouhealth_ui) (/ (Variables|Default|GetHP) (Variables|Default|GetMAX%20HP))))