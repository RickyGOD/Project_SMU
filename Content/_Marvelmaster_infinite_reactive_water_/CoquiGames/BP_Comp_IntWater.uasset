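; Actor component that makes its owner interact with the reactive water system, with optional physics and buoyancy.
; On first Tick, used so static meshes support it, it adds a local or standard water tag to the owner and its components, then registers with GlobalUpdater_BP.
; It can enable physics on the owner's static mesh and float it via BuoyancyFunction every frame, disabling Tick when buoyancy is off.
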(event EventTick
  (params (DeltaSeconds :type Float%20%28single-precision%29))
  (bind _returnvalue (Components|GetOwner))
  (bind _returnvalue_2 (Actor|GetComponentbyClass _returnvalue "/Script/Engine.StaticMeshComponent"))
  ;[1 1 1] Use Tick to allow static meshes to use this component
  (Utilities|FlowControl|Sequence
    (:then_0
      ;[1 1 1] Add tags and register actor with GlobalUpdater
      (Utilities|FlowControl|DoOnce false
        (:Completed
          (CallFunction|FnAddTags)
          (CallFunction|FnRegisterActor))))
    (:then_1
      (Utilities|FlowControl|DoOnce false
        (:Completed
          (if (Variables|Setup|GetSimulatePhysics)
            (Physics|SetSimulatePhysics (Actor|GetComponentbyClass (Components|GetOwner) "/Script/Engine.StaticMeshComponent") true)))))
    (:then_2
      (if (Variables|Setup|GetAddBuoyancy)
        (Utilities|IsValid _returnvalue_2
          (:Is%20Valid
            (CallFunction|BuoyancyFunction _returnvalue_2 (Variables|Setup|GetBuoyancyStarts) "ObjectTypeQuery7")))))
    (:then_3
      (if (not (Variables|Setup|GetAddBuoyancy))
        ;[1 1 1] Disable Tick
        (Components|Tick|SetComponentTickEnabled false)))))

(fn FnRegisterActor
  (bind _outactors (Actor|GetAllActorsOfClass "/Game/_Marvelmaster_infinite_reactive_water_/CoquiGames/GlobalUpdater_BP.GlobalUpdater_BP_C"))
  (Utilities|IsValid (Utilities|Array|Get(acopy) _outactors)
    (:Is%20Valid
      (LocalVariables|SetUpdater (Utilities|Array|Get(acopy) _outactors))
      (Default|FnRegisterActor (LocalVariables|GetUpdater) (Components|GetOwner)))))

(fn FnAddTags
  (if (Variables|Setup|GetUseWaterLocal)
    (Utilities|FlowControl|Sequence
      (:then_0
        (Utilities|Array|AddUnique (Variables|/Script/Engine.Actor|GetTags (Components|GetOwner)) (Variables|Setup|GetLocalWaterTag)))
      (:then_1
        (for _array_element (Actor|GetComponentsByClass (Components|GetOwner) "/Script/Engine.SkeletalMeshComponent")
          (Utilities|Array|AddUnique (Variables|/Script/Engine.ActorComponent|GetComponentTags _array_element) (Variables|Setup|GetLocalWaterTag))))
      (:then_2
        (for _array_element_2 (Actor|GetComponentsByClass (Components|GetOwner) "/Script/Engine.PrimitiveComponent")
          (Utilities|Array|AddUnique (Variables|/Script/Engine.ActorComponent|GetComponentTags _array_element_2) (Variables|Setup|GetLocalWaterTag)))))
    (else
      (Utilities|FlowControl|Sequence
        (:then_0
          (Utilities|Array|AddUnique (Variables|/Script/Engine.Actor|GetTags (Components|GetOwner)) (Variables|Setup|GetWaterTag)))
        (:then_1
          (for _array_element_3 (Actor|GetComponentsByClass (Components|GetOwner) "/Script/Engine.SkeletalMeshComponent")
            (Utilities|Array|AddUnique (Variables|/Script/Engine.ActorComponent|GetComponentTags _array_element_3) (Variables|Setup|GetWaterTag))))
        (:then_2
          (for _array_element_4 (Actor|GetComponentsByClass (Components|GetOwner) "/Script/Engine.PrimitiveComponent")
            (Utilities|Array|AddUnique (Variables|/Script/Engine.ActorComponent|GetComponentTags _array_element_4) (Variables|Setup|GetWaterTag))))))))