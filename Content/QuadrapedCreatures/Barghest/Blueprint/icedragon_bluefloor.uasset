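; Blue floor hazard actor, apparently for an ice dragon encounter, that damages the Zhanshi-BP character.
; When its collision component begins overlapping, it checks an IsBluefloor flag on a referenced object, then applies a small fixed damage if the other actor casts to Zhanshi-BP.
; A bluefloor_block event toggles the floor's visibility, makes it block all channels and sets its collision component to overlap all channels.
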(event OnComponentBeginOverlap(bluefloor_collision)
  (params (OverlappedComponent :type Primitive%20Component%20Object%20Reference) (OtherActor :type Actor%20Object%20Reference) (OtherComp :type Primitive%20Component%20Object%20Reference) (OtherBodyIndex :type Integer) (bFromSweep :type Boolean) (SweepResult :type Hit%20Result%20Structure%20%28by%20ref%29))
  (bind _output_get (Variables|Default|Setis%20bluefloor (Variables|/Game/MalbersAnimations/icedragon/icedragon.icedragon_C|Getis%20bluefloor (Variables|Default|GetNewVar_1))))
  (if _output_get
    (bind _aszhanshi__bp (Utilities|Casting|CastToZhanshi-BP OtherActor))
    (Game|Damage|ApplyDamage _aszhanshi__bp 1e+01 0 0)))

(event Custom|bluefloor_block
  (Rendering|ToggleVisibility (Variables|Default|Getbluefloor) false)
  (Collision|SetCollisionResponsetoAllChannels (Variables|Default|Getbluefloor) "ECR_Block")
  (Collision|SetCollisionResponsetoAllChannels (Variables|Default|Getbluefloor_collision) "ECR_Overlap"))

(event EventBeginPlay)

(event Collision|EventActorBeginOverlap
  (params (OtherActor :type Actor%20Object%20Reference)))

(event EventTick
  (params (DeltaSeconds :type Float%20%28single-precision%29)))

(fn ConstructionScript)