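; BP_DamgeBox is a one-shot damage actor that applies a small hit to a pawn at its spawn location.
; On BeginPlay it runs a zero-length single box trace for Pawn objects, centered slightly below the actor, with timed debug drawing.
; It applies damage to the hit actor without checking the trace result, then immediately destroys itself.
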(event EventBeginPlay
  (bind _returnvalue (Transformation|GetActorLocation))
  (bind (_x _y _z) (Math|Vector|BreakVector _returnvalue))
  (bind _outhit (Class|KismetSystemLibrary|BoxTraceSingleforObjects (Math|Vector|MakeVector _x _y (- _z 5e+01)) (Math|Vector|MakeVector _x _y (- _z 5e+01)) "100.000000,100.000000,100.000000" "0, 0, 0" (Utilities|Array|MakeArray "ObjectTypeQuery3") false 0 "ForDuration" true))
  (Game|Damage|ApplyDamage (.HitActor (Collision|BreakHitResult _outhit)) 0.5 0 0)
  (Actor|DestroyActor))

(event Collision|EventActorBeginOverlap
  (params (OtherActor :type Actor%20Object%20Reference)))

(event EventTick
  (params (DeltaSeconds :type Float%20%28single-precision%29)))

(fn ConstructionScript)