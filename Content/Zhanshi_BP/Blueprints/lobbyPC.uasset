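; Lobby player controller that runs each player's lobby menu and relays their character choice to the game mode.
; Player settings updates go to lobbyGM, which swaps the character and triggers a lobby-wide update.
; Other events refresh the player list and count in the menu widget or replace it with a loading screen.
; Being kicked opens the main menu and destroys the session, as does EndPlay; the save check is an empty stub.
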(event Custom|intalsetup
  ;[1 1 1] inital setup/ check
  (CallFunction|Savegamecheck)
  (CallFunction|Callupdate (Variables|playerinfo|Getplayersetting) false))

(event Custom|setuplobbymenu
  (params (survername :type Text))
  (Variables|Default|SetbShowMouseCursor true)
  (bind _returnvalue (UserInterface|CreateWidget "/Game/UI/UI/lobbymenu.lobbymenu_C" 0 survername))
  (bind _output_get (Variables|widgets|SetlobbymenuWB _returnvalue))
  (UserInterface|Viewport|AddtoViewport _output_get 0))

(event Custom|callupdate
  (params (playerinfo :type Playerinfo%20Structure) (changestatus :type Boolean))
  (bind _returnvalue (Game|GetGameMode))
  (bind _aslobby_gm (Utilities|Casting|CastTolobbyGM _returnvalue))
  ;[1 1 1] assigns update character selection/tells everyone to update lobby
  (Variables|playerinfo|Setplayersetting playerinfo)
  (Default|Swapcharacter _aslobby_gm self (.myplayercharacter (Variables|playerinfo|Getplayersetting)) changestatus)
  (Default|Everyupdate _aslobby_gm))

(event Custom|addplayerinfo
  (params (conncetedplayerinfo :type Array%20of%20Playerinfo%20Structures))
  (bind _lobbymenuwb (Variables|widgets|GetlobbymenuWB))
  ;[1 1 1] update player list
  (Variables|Default|Setallcontectplayers conncetedplayerinfo)
  (Utilities|IsValid _lobbymenuwb
    (:Is%20Valid
      (Default|Cleanplayerlist _lobbymenuwb)
      (for _array_element (Variables|Default|Getallcontectplayers)
        (Default|Updateplayerwindwn (Variables|widgets|GetlobbymenuWB) _array_element)))))

(event Custom|showloadingscreen
  (Widget|RemovefromParent (Variables|widgets|GetlobbymenuWB))
  (bind _returnvalue (UserInterface|CreateWidget "/Game/UI/UI/loadingui.loadingui_C" self))
  (UserInterface|Viewport|AddtoViewport _returnvalue 0))

(event Custom|updatenumberofplayers
  (params (currentplayers :type Integer) (maxplayers :type Integer))
  (bind _lobbymenuwb (Variables|widgets|GetlobbymenuWB))
  ;[1 1 1] update
  (Utilities|IsValid _lobbymenuwb
    (:Is%20Valid
      (Variables|/Game/UI/UI/lobbymenu.lobbymenu_C|Setplayerdisplay _lobbymenuwb (Utilities|Text|FormatText "{currentplayers}of {MAXplayers}" currentplayers maxplayers)))))

(event Custom|Kicked
  (Game|OpenLevel(byName) "mainmenu")
  (|DestroySession self))

(event EventEndPlay
  (params (EndPlayReason :type EEndPlayReason%20Enum :default "Destroyed"))
  (|DestroySession self))

(fn ConstructionScript)

(fn Savegamecheck)