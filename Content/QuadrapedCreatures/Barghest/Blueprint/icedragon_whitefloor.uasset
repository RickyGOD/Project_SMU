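; An ice dragon "white floor" hazard that periodically damages the Zhanshi-BP character after it overlaps the floor's collision.
; On overlap it finds the first Icedragon and, while that dragon's IsWhitefloor flag is set, applies damage in a delayed loop with no end-overlap check.
; The whitefloor_block event toggles the floor mesh's visibility, makes it blocking and sets the trigger to overlap.
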(event OnComponentBeginOverlap(whitefloor_collision)
  (params (OverlappedComponent :type Primitive%20Component%20Object%20Reference) (OtherActor :type Actor%20Object%20Reference) (OtherComp :type Primitive%20Component%20Object%20Reference) (OtherBodyIndex :type Integer) (bFromSweep :type Boolean) (SweepResult :type Hit%20Result%20Structure%20%28by%20ref%29))
  (bind _outactors (Actor|GetAllActorsOfClass "/Game/MalbersAnimations/icedragon/icedragon.icedragon_C"))
  (if (Variables|/Game/MalbersAnimations/icedragon/icedragon.icedragon_C|Getis%20whitefloor (Utilities|Array|Get(acopy) _outactors)) :!label _label
    (bind _aszhanshi__bp (Utilities|Casting|CastToZhanshi-BP OtherActor))
    (Game|Damage|ApplyDamage _aszhanshi__bp 1e+01 0 0)
    (Utilities|FlowControl|Delay 3.0)
    (goto _label)))

(event Custom|whitefloor_block
  (Rendering|ToggleVisibility (Variables|Default|Getwhitefloor) false)
  (Collision|SetCollisionResponsetoAllChannels (Variables|Default|Getwhitefloor) "ECR_Block")
  (Collision|SetCollisionResponsetoAllChannels (Variables|Default|Getwhitefloor_collision) "ECR_Overlap"))

(event EventBeginPlay)

(event Collision|EventActorBeginOverlap
  (params (OtherActor :type Actor%20Object%20Reference)))

(event EventTick
  (params (DeltaSeconds :type Float%20%28single-precision%29)))

(fn ConstructionScript)