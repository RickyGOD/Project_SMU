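; Gargo enemy character that runs the Gargo_BH behavior tree and attacks the player with a montage and waterball projectiles.
; Pawn sensing latches the first sighting of the player and writes the "seen player" and "player" blackboard keys.
; The attack event faces the player, plays the montage, waits its length, then calls back into the attack task.
; The waterball event spawns a Waterball at the right hand, aimed at the player.
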(event OnSeePawn(PawnSensing)
  (params (Pawn :type Pawn%20Object%20Reference))
  (bind _returnvalue (AI|GetBlackboard 0))
  (if (and (== Pawn (Game|Player|GetPlayerPawn 0)) (not (Variables|Default|Getseen%20player)))
    (Variables|Default|Setseen%20player true)
    (AI|Components|Blackboard|SetValueasBool _returnvalue (Utilities|Name|MakeLiteralName "seen player") false)
    (AI|Components|Blackboard|SetValueasObject _returnvalue (Utilities|Name|MakeLiteralName "player") Pawn)))

(event Custom|gargo_attack
  (params (task_gargo_attack :type Gargo%20Attack%20Object%20Reference))
  (Transformation|SetActorRotation (Math|Rotator|FindLookatRotation (Transformation|GetActorLocation) (Transformation|GetActorLocation (Game|GetPlayerCharacter 0))))
  (Variables|Default|Setanimation%20montage "/Game/DragonsPackage/Gargo/montage/gargo_attack.gargo_attack")
  (Animation|PlayAnimMontage (Variables|Default|Getanimation%20montage) 1.0 "None")
  (Utilities|FlowControl|Delay (Variables|/Script/Engine.AnimSequenceBase|GetSequenceLength (Variables|Default|Getanimation%20montage)))
  (CallFunction|GargoAttack task_gargo_attack))

(event Custom|waterball
  (bind _righthand_collision (Variables|Default|GetRightHand_collision))
  (bind _returnvalue (Transformation|GetWorldLocation _righthand_collision))
  (Game|SpawnActorfromClass "/Game/DragonsPackage/Gargo/Blueprint/waterball.waterball_C" (Math|Transform|MakeTransform _returnvalue (Math|Rotator|FindLookatRotation _returnvalue (Transformation|GetActorLocation (Game|GetPlayerCharacter 0)))) "Undefined" 0 0))

(event EventBeginPlay
  (AI|RunBehaviorTree (AI|GetAIController self) "/Game/DragonsPackage/Gargo/Blueprint/Gargo_BH.Gargo_BH"))

(fn ConstructionScript)