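; Behavior tree task for the Barghest creature that checks whether the player is within attack distance.
; On execute, it measures the distance between the controlled pawn and the Player blackboard actor and compares it to the Attackrange blackboard float.
; It writes the result to the Inattackrange blackboard bool and always finishes successfully, whether or not the player is in range.
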(event EventReceiveExecuteAI
  (params (OwnerController :type AI%20Controller%20Object%20Reference) (ControlledPawn :type Pawn%20Object%20Reference))
  (Class|BTFunctionLibrary|SetBlackboardValueasBool (Variables|Default|Getinattackrange) (<= (Math|Vector|VectorLength (- (Transformation|GetActorLocation ControlledPawn) (Transformation|GetActorLocation (AI|BehaviorTree|GetBlackboardValueasActor (Variables|Default|Getplayer))))) (Class|BTFunctionLibrary|GetBlackboardValueasFloat (Variables|Default|Getattackrange))))
  (AI|BehaviorTree|FinishExecute true))