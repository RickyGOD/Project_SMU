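; A trigger volume that slows the Zhanshi-BP warrior while inside it and sets off a gargoyle encounter.
; On box begin overlap by any actor, it calls SpawnGargo and BluewallBlock on the first Spawn_gargo and Jizhi02_bluewall actors found in the level.
; It then casts the overlapping actor to Zhanshi-BP to call SlowDown, and calls SlowDownOut when that actor leaves.
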(event OnComponentBeginOverlap(Box)
  (params (OverlappedComponent :type Primitive%20Component%20Object%20Reference) (OtherActor :type Actor%20Object%20Reference) (OtherComp :type Primitive%20Component%20Object%20Reference) (OtherBodyIndex :type Integer) (bFromSweep :type Boolean) (SweepResult :type Hit%20Result%20Structure%20%28by%20ref%29))
  (bind _outactors (Actor|GetAllActorsOfClass "/Game/MalbersAnimations/icedragon/jizhi02/spawn_gargo.spawn_gargo_C"))
  (Default|SpawnGargo (Utilities|Array|Get(acopy) _outactors))
  (bind _outactors_2 (Actor|GetAllActorsOfClass "/Game/MalbersAnimations/icedragon/jizhi02/jizhi02_bluewall.jizhi02_bluewall_C"))
  (Default|BluewallBlock (Utilities|Array|Get(acopy) _outactors_2))
  (bind _aszhanshi__bp (Utilities|Casting|CastToZhanshi-BP OtherActor))
  (Default|SlowDown _aszhanshi__bp))

(event OnComponentEndOverlap(Box)
  (params (OverlappedComponent :type Primitive%20Component%20Object%20Reference) (OtherActor :type Actor%20Object%20Reference) (OtherComp :type Primitive%20Component%20Object%20Reference) (OtherBodyIndex :type Integer))
  (bind _aszhanshi__bp (Utilities|Casting|CastToZhanshi-BP OtherActor))
  (Default|SlowDownOut _aszhanshi__bp))

(event EventBeginPlay)

(event Collision|EventActorBeginOverlap
  (params (OtherActor :type Actor%20Object%20Reference)))

(event EventTick
  (params (DeltaSeconds :type Float%20%28single-precision%29)))

(fn ConstructionScript)