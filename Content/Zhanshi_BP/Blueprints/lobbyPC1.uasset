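; Lobby player controller that manages a player's lobby menu, character selection and session exit in a multiplayer game.
; Selections resolve through the lobbyGM character list into player info, then the GameMode swaps the character and refreshes everyone.
; Update events feed the player list, player count and character button availability, while others show loading or handle kicks with session teardown.
; Save functions are empty stubs, and a stray event resets an IceDragon boss bar.
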(event Custom|intalsetup
  ;[1 1 1] inital setup/ check
  (CallFunction|Savegamecheck)
  (CallFunction|Callupdate (Variables|playerinfo|Getplayersetting) false))

(event Custom|setuplobbymenu
  (params (survername :type Text))
  (Variables|Default|SetbShowMouseCursor true)
  (bind _returnvalue (UserInterface|CreateWidget "/Game/UI/UI/lobbymenu.lobbymenu_C" 0 survername))
  (bind _output_get (Variables|widgets|SetlobbymenuWB _returnvalue))
  (UserInterface|Viewport|AddtoViewport _output_get 0))

(event Custom|updateavaiblecharacter
  (params (avaiblecharacter :type Array%20of%20Booleans)))

(event Custom|UpdateBossUI
  (Progress|SetPercent (Variables|/Game/UI/HPUI/icedragonhealthUI.icedragonhealthUI_C|GetProgressBar_145 (Variables|Default|GetIceDragonUI)) 0.0))

(event Custom|callupdate
  (params (playerinfo :type Playerinfo%20Structure) (changestatus :type Boolean))
  (bind _returnvalue (Game|GetGameMode))
  (bind _aslobby_gm (Utilities|Casting|CastTolobbyGM _returnvalue))
  ;[1 1 1] assigns update character selection/tells everyone to update lobby
  (Variables|playerinfo|Setplayersetting playerinfo)
  (Default|Swapcharacter _aslobby_gm self (.myplayercharacter (Variables|playerinfo|Getplayersetting)) changestatus)
  (Default|Everyupdate _aslobby_gm))

(event Custom|addplayerinfo
  (params (conncetedplayerinfo :type Array%20of%20Playerinfo%20Structures))
  (bind _lobbymenuwb (Variables|widgets|GetlobbymenuWB))
  ;[1 1 1] update player list
  (Variables|Default|Setallcontectplayers conncetedplayerinfo)
  (Utilities|IsValid _lobbymenuwb
    (:Is%20Valid
      (Default|Cleanplayerlist _lobbymenuwb)
      (for _array_element (Variables|Default|Getallcontectplayers)
        (Default|Updateplayerwindwn (Variables|widgets|GetlobbymenuWB) _array_element)))))

(event Custom|showloadingscreen
  (Widget|RemovefromParent (Variables|widgets|GetlobbymenuWB))
  (bind _returnvalue (UserInterface|CreateWidget "/Game/UI/UI/loadingui.loadingui_C" self))
  (UserInterface|Viewport|AddtoViewport _returnvalue 0))

(event Custom|updatenumberofplayers
  (params (currentplayers :type Integer) (maxplayers :type Integer))
  (bind _lobbymenuwb (Variables|widgets|GetlobbymenuWB))
  ;[1 1 1] update
  (Utilities|IsValid _lobbymenuwb
    (:Is%20Valid
      (Variables|/Game/UI/UI/lobbymenu.lobbymenu_C|Setplayerdisplay _lobbymenuwb (Utilities|Text|FormatText "{currentplayers}of {MAXplayers}" currentplayers maxplayers)))))

(event Custom|Kicked
  (Game|OpenLevel(byName) "mainmenu")
  (|DestroySession self))

(event Custom|updateavaivlechararcter
  (params (avaiblecharacter :type Array%20of%20Booleans))
  (bind _lobbymenuwb (Variables|widgets|GetlobbymenuWB))
  (Variables|Default|Setavaiblecharacter avaiblecharacter)
  (Utilities|IsValid _lobbymenuwb
    (:Is%20Valid
      (for (_array_element _array_index) (Variables|/Game/UI/UI/characterselect.characterselect_C|Getcharacterbutton (Variables|/Game/UI/UI/lobbymenu.lobbymenu_C|Getcharacterselect _lobbymenuwb))
        (Widget|SetIsEnabled _array_element (not (Utilities|Array|Get(acopy) (Variables|Default|Getavaiblecharacter) _array_index)))))))

(event Custom|assignselectchararcter
  (params (characterID :type Integer) (characteriamge :type Texture%202D%20Object%20Reference))
  (Variables|Default|Setselectcharacter characterID)
  (Variables|Default|Setcharacterimage characteriamge)
  (Variables|Default|Setpreviousselection (Variables|Default|Getselectcharacter))
  (CallFunction|ChareacterCheck)
  (Development|PrintString (Utilities|String|Append "UI:" (Utilities|String|ToString(Integer) characterID)) true true "(R=1.000000,G=0.000000,B=0.071131,A=1.000000)"))

(event Custom|assignplayer
  (params (character :type Character%20Class%20Reference) (characteriamge :type Texture%202D%20Object%20Reference))
  (Utilities|Struct|Setmembersinplayerinfo (Variables|playerinfo|Getplayersetting) character characteriamge)
  (CallFunction|Savegame)
  (CallFunction|Callupdate))

(event EventBeginPlay)

(event EventEndPlay
  (params (EndPlayReason :type EEndPlayReason%20Enum :default "Destroyed"))
  (|DestroySession self))

(fn ConstructionScript)

(fn Savegamecheck)

(fn ChareacterCheck
  (CallFunction|Assignplayer (Utilities|Array|Get(acopy) (Variables|/Game/Zhanshi_BP/Blueprints/lobbyGM.lobbyGM_C|Getcharacters (.AsLobby%20GM (Utilities|Casting|CastTolobbyGM (Game|GetGameMode)))) (Variables|Default|Getselectcharacter)) (Variables|Default|Getcharacterimage)))

(fn Savegame)