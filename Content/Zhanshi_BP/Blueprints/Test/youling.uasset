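; Ghost (youling) enemy AI that wanders and damages the Zhanshi-BP warrior on contact.
; It walks to random nearby reachable points, re-rolled through a 3-second Delay on Tick, and speeds up toward the player's location when PawnSensing sees a pawn.
; Overlapping the warrior starts a half-second TakeDamage2 loop, which stops when any overlap ends.
; A box-trace ApplyDamage loop is left unconnected.
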(event OnSeePawn(PawnSensing)
  (params (Pawn :type Pawn%20Object%20Reference))
  ;[1 1 1] 看到角色
  (CallFunction|AiGo))

(event Custom|ai_random
  (bind _self self)
  ;[1 1 1] ai随机移动
  (Variables|Default|SetMaxWalkSpeed 2e+02)
  (AI|AIMoveTo _self 0 (.RandomLocation (AI|Navigation|GetRandomReachablePointinRadius (Transformation|GetActorLocation _self) 5e+02 0 0)) 0 5.0 false))

(event Custom|ai_go
  ;[1 1 1] 冲刺
  (Variables|Default|SetMaxWalkSpeed 4e+02)
  (AI|AIMoveTo self (Transformation|GetActorLocation (Game|GetPlayerCharacter 0)) 0 5.0 false))

(event EventBeginPlay
  ;[1 1 1] 执行运动
  (CallFunction|AiRandom))

(event Collision|EventActorBeginOverlap
  (params (OtherActor :type Actor%20Object%20Reference))
  (bind _aszhanshi__bp (Utilities|Casting|CastToZhanshi-BP OtherActor))
  (Variables|Default|SetIsInVolume true)
  (Default|TakeDamage2% _aszhanshi__bp :!label _label)
  (if (Variables|Default|GetIsInVolume)
    (Utilities|FlowControl|Delay 0.5)
    (goto _label)))

(event EventTick
  (params (DeltaSeconds :type Float%20%28single-precision%29))
  ;[1 1 1] 间隔时间自己走动
  (Utilities|FlowControl|Delay 3.0)
  (CallFunction|AiRandom))

(event Collision|EventActorEndOverlap
  (params (OtherActor :type Actor%20Object%20Reference))
  (Variables|Default|SetIsInVolume false))

(fn ConstructionScript)