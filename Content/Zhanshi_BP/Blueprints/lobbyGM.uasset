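; Lobby game mode that tracks joining players, manages their pawns and server-travels everyone to the game map.
; PostLogin records controllers and gives players after the first a Zhanshi pawn at a fixed location.
; Respawn and character-swap events use random spawn points; respawn calls Everyupdate to share player settings and set start readiness.
; Spawn-point and lobby initialization is disconnected, and the kick-list and cannot-start events are empty.
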(event Custom|everyupdate
  (bind _allplayercontrollers (Variables|serversetting|Getallplayercontrollers))
  (bind _output_get (Variables|serversetting|Setcurrentplayers (Utilities|Array|Length (Variables|serversetting|Getallplayercontrollers))))
  (if (> _output_get 0)
    (Utilities|Array|Clear (Variables|serversetting|Getconnectplayers))
    (for _array_element _allplayercontrollers
      (bind _aslobby_pc1 (Utilities|Casting|CastTolobbyPC1 _array_element))
      (Utilities|Array|Add (Variables|serversetting|Getconnectplayers) (Variables|/Game/Zhanshi_BP/Blueprints/lobbyPC1.lobbyPC1_C|Getplayersetting _aslobby_pc1))
      (Default|Updatenumberofplayers _aslobby_pc1 (Variables|serversetting|Getcurrentplayers) (Variables|serversetting|GetMAXplayers)))
    (for _array_element_2 _allplayercontrollers
      (bind _aslobby_pc1_2 (Utilities|Casting|CastTolobbyPC1 _array_element_2))
      (Default|Addplayerinfo _aslobby_pc1_2 (Variables|serversetting|Getconnectplayers))
      (Default|Updateavaivlechararcter _aslobby_pc1_2 (Variables|serversetting|Getavaivlecharacter))
      (CallFunction|Addtokicklist))
    (bind _array_element_3 (Utilities|Array|ForEachLoopwithBreak (Variables|serversetting|Getconnectplayers))
      (:LoopBody
        (if (== (.myplayercharacter (Utilities|Struct|Breakplayerinfo _array_element_3)) "/Game/Maps/daoju/1-chuan.1-chuan_C")
          (Variables|serversetting|Setcanwestart? false)
          (CallFunction|Cannotstartgame)
          (else
            (Variables|serversetting|Setcanwestart? true)))))))

(event Custom|swapcharacter
  (params (playercontroller :type Player%20Controller%20Object%20Reference) (characterclass :type Character%20Class%20Reference) (changestatus :type Boolean))
  (bind _returnvalue (Pawn|GetControlledPawn playercontroller))
  (bind _spawnpoints (Variables|serversetting|Getspawnpoints))
  (if (not changestatus)
    (Utilities|IsValid _returnvalue
      (:Is%20Valid
        (Actor|DestroyActor _returnvalue)
        (bind _returnvalue_2 (Game|SpawnActorfromClass characterclass (Transformation|GetActorTransform (Utilities|Array|Get(acopy) _spawnpoints (Math|Random|RandomIntegerinRange 0 (- (Utilities|Array|Length _spawnpoints) 1)))) "Undefined" 0 0))
        (Pawn|Possess playercontroller _returnvalue_2)))))

(event Custom|launchthegame
  (Development|ExecuteConsoleCommand "servertravel /game/Maps/1" (Game|GetPlayerController 0)))

(event Custom|respawnplayer
  (params (playercontroller :type Player%20Controller%20Object%20Reference))
  (bind _returnvalue (Pawn|GetControlledPawn playercontroller))
  (bind _spawnpoints (Variables|serversetting|Getspawnpoints))
  (Utilities|IsValid _returnvalue
    (:Is%20Valid
      (Actor|DestroyActor _returnvalue))
    (:Is%20Not%20Valid
      _))
  (bind _returnvalue_2 (Game|SpawnActorfromClass "/Game/Zhanshi_BP/Blueprints/Zhanshi-BP.Zhanshi-BP_C" (Transformation|GetActorTransform (Utilities|Array|Get(acopy) _spawnpoints (Math|Random|RandomIntegerinRange 0 (- (Utilities|Array|Length _spawnpoints) 1)))) "Undefined" 0 0))
  (Pawn|Possess playercontroller _returnvalue_2)
  (CallFunction|Everyupdate))

(event Custom|addtokicklist)

(event Custom|cannotstartgame)

(event EventBeginPlay)

(event EventPostLogin
  (params (NewPlayer :type Player%20Controller%20Object%20Reference))
  (bind _allplayercontrollers (Variables|serversetting|Getallplayercontrollers))
  (Utilities|Array|Add _allplayercontrollers 0)
  (if (> (Utilities|Array|Length _allplayercontrollers) 1)
    (bind _returnvalue (Game|SpawnActorfromClass "/Game/Zhanshi_BP/Blueprints/Zhanshi-BP.Zhanshi-BP_C" (Math|Transform|MakeTransform "0, 0,500.000000" "0, 0, 0" "1,1,1") "AlwaysSpawn" 0 0))
    (Pawn|Possess NewPlayer _returnvalue)))

(fn ConstructionScript)