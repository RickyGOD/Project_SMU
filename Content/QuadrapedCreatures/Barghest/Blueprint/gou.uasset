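; Barghest enemy character with behavior-tree AI that spots the tagged player, attacks, takes damage and dies.
; BeginPlay attaches a weapon and fills the blackboard; pawn sensing flags the player and sets chase speed.
; Attacks play one of two random montages, with a notify-driven box trace applying damage.
; Hits read the player's attack state to pick damage, update the health widget and trigger death; lock-on targeting toggles an icon.
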(event OnSeePawn(PawnSensing)
  (params (Pawn :type Pawn%20Object%20Reference))
  (bind _returnvalue (AI|GetBlackboard 0))
  ;[1 1 1] 看到玩家和把seen player和player变量获取到行为树
  (if (Actor|ActorHasTag Pawn "zhanshi tag")
    (Variables|Default|Setseen%20player true)
    (AI|Components|Blackboard|SetValueasBool _returnvalue (Utilities|Name|MakeLiteralName "seen player") true)
    (AI|Components|Blackboard|SetValueasObject _returnvalue (Utilities|Name|MakeLiteralName "player") Pawn)
    (Variables|/Script/Engine.CharacterMovementComponent|SetMaxWalkSpeed (Variables|Character|GetCharacterMovement) 4e+02)))

(event Custom|attacknotify
  (bind _returnvalue (Transformation|GetActorLocation))
  ;[1 1 1] 攻击伤害
  (bind _outhit (Class|KismetSystemLibrary|BoxTraceSingleforObjects _returnvalue (+ _returnvalue (* (Transformation|GetActorForwardVector) (Variables|Default|Getattackdistance))) "200.000000,140.000000,90.000000" "0, 0, 0" (Utilities|Array|MakeArray "ObjectTypeQuery3") false 0 "None" true))
  (Game|Damage|ApplyDamage (.HitActor (Collision|BreakHitResult _outhit)) (Variables|Default|Getattackdamage) 0 self))

(event Custom|on%20death
  ;[1 1 1] 死亡
  (bind _returnvalue (Animation|GetCurrentMontage :!class /Script/Engine.Character))
  (Utilities|IsValid _returnvalue
    (:Is%20Valid
      (Animation|StopAnimMontage _returnvalue))
    (:Is%20Not%20Valid
      _))
  (Variables|Default|SetIs%20dead true)
  (AI|Components|Blackboard|SetValueasBool (AI|GetBlackboard 0) (Utilities|Name|MakeLiteralName "Is dead") true)
  (Collision|SetCollisionEnabled (Variables|Collision|GetCapsuleComponent) "NoCollision")
  (Utilities|FlowControl|Delay 7.0)
  (Actor|DestroyActor))

(event Custom|attacks
  (params (attack :type GB%20Ltask%20Attack%20Object%20Reference))
  ;[1 1 1] 攻击事件
  (Transformation|SetActorRotation (Math|Rotator|FindLookatRotation (Transformation|GetActorLocation) (Transformation|GetActorLocation (Game|GetPlayerCharacter 0))))
  (switch int (Math|Random|RandomIntegerinRange 0 1)
    (:0
      (Variables|Default|Setattack%20montage "/Game/ai/content/Enemy_Troll/Enemy_Troll_Poison_Animation/GBL_Troll_Attack_Charge_Montage.GBL_Troll_Attack_Charge_Montage"))
    (:1
      (Variables|Default|Setattack%20montage "/Game/ai/content/Enemy_Troll/Enemy_Troll_Poison_Animation/GBL_Troll_Attack_Overhead_Montage.GBL_Troll_Attack_Overhead_Montage")))
  (Animation|PlayAnimMontage (Variables|Default|Getattack%20montage) 1.0 "None")
  (Utilities|FlowControl|Delay (Variables|/Script/Engine.AnimSequenceBase|GetSequenceLength (Variables|Default|Getattack%20montage)))
  (Default|Onattack attack))

(event EventDamage
  (params (Aistate :type A%20Istate%20Structure) (Hitnumber :type Integer) (mageAistate :type Mage%20A%20Istate%20Structure) (GBLAistate :type GBLA%20Istate%20Structure) (BearAistate :type Bear%20A%20Istate%20Structure) (JYGAistate :type JYGA%20Istate%20Structure) (LXCAistate :type LXCA%20Istate%20Structure) (island1Aistate :type Island%201A%20Istate%20Structure) (island2Aistate :type Island%202A%20Istate%20Structure) (gouAistate :type Gou%20A%20Istate%20Structure))
  ;[1 1 1 1 50] 受伤判断
  ;;[1 1 1] 判断具体攻击行为
  (bind _aszhanshi__bp (Utilities|Casting|CastToZhanshi-BP (Game|GetPlayerCharacter 0)))
  (if (Variables|/Game/Zhanshi_BP/Blueprints/Zhanshi-BP.Zhanshi-BP_C|GetIsGreatSword? _aszhanshi__bp)
    ;;[1 1 1] 左键伤害
    (switch int (Variables|/Game/Zhanshi_BP/Blueprints/Zhanshi-BP.Zhanshi-BP_C|GetNumber _aszhanshi__bp)
      (:0
        _)
      (:1
        _)
      (:2
        _)
      (:3
        _))
    (bind _damage (Default|StuckZhanShi _aszhanshi__bp "2Lattack"))
    (Utilities|SHSZ _damage)
    (elif (Variables|/Game/Zhanshi_BP/Blueprints/Zhanshi-BP.Zhanshi-BP_C|Getleftkey _aszhanshi__bp)
      ;;[1 1 1] 左键伤害
      (switch int (Variables|/Game/Zhanshi_BP/Blueprints/Zhanshi-BP.Zhanshi-BP_C|GetNumber _aszhanshi__bp)
        (:0
          _)
        (:1
          _)
        (:2
          _)
        (:3
          _))
      (bind _damage_2 (Default|StuckZhanShi _aszhanshi__bp "1Lattack"))
      (Utilities|SHSZ _damage_2)
      (elif (Variables|/Game/Zhanshi_BP/Blueprints/Zhanshi-BP.Zhanshi-BP_C|GetUsing%20SKILL _aszhanshi__bp)
        (if (Variables|/Game/Zhanshi_BP/Blueprints/Zhanshi-BP.Zhanshi-BP_C|GetE-Skill _aszhanshi__bp)
          ;;[1 1 1] E技能伤害
          (bind _skilldamage (Default|StuckZhanShi _aszhanshi__bp "ESkill"))
          (Utilities|SHSZ _skilldamage)
          (elif (Variables|/Game/Zhanshi_BP/Blueprints/Zhanshi-BP.Zhanshi-BP_C|GetDunchong _aszhanshi__bp)
            (bind _skilldamage_2 (Default|StuckZhanShi _aszhanshi__bp "Dunchong"))
            (Utilities|SHSZ _skilldamage_2)
            (else
              ;;[1 1 1] Q技能伤害
              (bind _skilldamage_3 (Default|StuckZhanShi _aszhanshi__bp "QSkill"))
              (Utilities|SHSZ _skilldamage_3))))
        (else
          ;;[1 1 1] 右键伤害
          (switch int (Variables|/Game/Zhanshi_BP/Blueprints/Zhanshi-BP.Zhanshi-BP_C|GetNumber _aszhanshi__bp)
            (:0
              _)
            (:1
              _)
            (:2
              _)
            (:3
              _))
          (bind _damage_3 (Default|StuckZhanShi _aszhanshi__bp "1Rattack"))
          (Utilities|SHSZ _damage_3)))))
  (CallFunction|UpdateWidget)
  ;;[1 1 1] 判断血量是否为0
  (Math|Float|CompareFloat (Variables|Default|Getgblhp) 0.0
    (:>
      (Animation|StopAnimMontage 0)
      ;;[1 1 1] 播放受伤动画
      (Animation|PlayAnimMontage (Utilities|Array|Get(acopy) (Utilities|Struct|BreakGBLAIstate GBLAistate)) 1.0 "None"))
    (:==
      (Utilities|FlowControl|DoOnce false :!label _label
        (:Completed
          (CallFunction|OnDeath))))
    (:<
      (goto _label))))

(event EventBeginPlay
  (bind _returnvalue (AI|GetBlackboard 0))
  ;[1 1 1] 血条
  (Variables|Default|Setgblhp (Variables|Default|Getgblmaxhp))
  (CallFunction|UpdateWidget)
  ;[1 1 1] weapon
  (bind _returnvalue_2 (Game|SpawnActorfromClass "/Game/ai/content/Enemy_Troll/Meshes/troll.troll_C" (Math|Transform|MakeTransform "0, 0, 0") "Undefined" 0 0))
  (Transformation|AttachComponentToComponent _returnvalue_2 (Variables|Character|GetMesh) "b_MF_Weapon_R_Socket" "KeepRelative" "KeepRelative" "KeepRelative" true)
  ;[1 1 1] 获取变量到行为树
  (AI|RunBehaviorTree (AI|GetAIController self) (Variables|Default|Getbehaviour%20tree))
  (AI|Components|Blackboard|SetValueasVector _returnvalue (Utilities|Name|MakeLiteralName "original location") (Transformation|GetActorLocation))
  (AI|Components|Blackboard|SetValueasFloat _returnvalue (Utilities|Name|MakeLiteralName "patrolradius") (Variables|Default|Getpatrolradius))
  (AI|Components|Blackboard|SetValueasFloat _returnvalue (Utilities|Name|MakeLiteralName "attackrange") (Variables|Default|Getattackrange))
  (AI|Components|Blackboard|SetValueasObject _returnvalue (Utilities|Name|MakeLiteralName "zhanshi") "/Game/Zhanshi_BP/Blueprints/Zhanshi-BP.Zhanshi-BP"))

(fn ConstructionScript)

(fn UpdateWidget
  (bind _asgblhealth_ui (Utilities|Casting|CastToGBLhealthUI (UserInterface|GetUserWidgetObject (Variables|Default|GetGBLWidget))))
  (Progress|SetPercent (Variables|/Game/UI/GBLhealthUI.GBLhealthUI_C|GetProgressBar_145 _asgblhealth_ui) (/ (Variables|Default|Getgblhp) (Variables|Default|Getgblmaxhp))))

(fn IsTargetable
  (return true))

(fn OnDeselected
  (Development|SetHiddeninGame (Variables|Default|GetlockIcon) true false)
  (return false))

(fn OnSelected
  (Development|SetHiddeninGame (Variables|Default|GetlockIcon) false false)
  (return false))